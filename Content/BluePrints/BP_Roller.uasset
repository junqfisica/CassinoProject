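; One six-faced roller of BP_SpinMachine, its parent actor, which spins and stops on the number the machine assigns by RollerId.
; After a start delay it spins on physics torque, then drops damping and records its angular speed.
; When allowed to stop and arrow alignment detects face zero, it disables physics and steps to the target angle at that speed, then calls RollerStopped.
; A DoOnce blocks respins until EnableSpin resets it.
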(event Custom|StopSpining
  (Class|PrimitiveComponent|SetAngularDamping (Variables|Default|GetRollerStaticMesh) 0.0)
  (bind _returnvalue (Class|PrimitiveComponent|GetPhysicsAngularVelocity (Variables|Default|GetRollerStaticMesh) "None"))
  (Variables|Spinning|SetCurrentAngularSpeed (Math|Float|Absolute(Float) (.y _returnvalue)))
  (Utilities|FlowControl|Sequence
    (:then_0
      ;[0.4754 1 0.9402] Set the angle based on the random number.
      (switch int (Variables|Result|GetRandomValue)
        (:0
          (Variables|Spinning|SetStopAtAngle 0))
        (:1
          (Variables|Spinning|SetStopAtAngle 60))
        (:2
          (Variables|Spinning|SetStopAtAngle 120))
        (:3
          (Variables|Spinning|SetStopAtAngle 180))
        (:4
          (Variables|Spinning|SetStopAtAngle 240))
        (:5
          (Variables|Spinning|SetStopAtAngle 300))))
    (:then_1
      (bind _returnvalue_2 (Utilities|Time|SetTimerbyEvent (delegate Custom|CheckForFaceZero) 0.01 true))
      (Variables|Spinning|SetCheckForFaceZeroTimerHandler _returnvalue_2))))

(event Custom|EnableSpin
  (bind _rollerstaticmesh (Variables|Default|GetRollerStaticMesh))
  (Utilities|FlowControl|DoOnce false) ; enters at Reset
)

(event Custom|GenerateRandomNumber
  (Variables|Random|SetTempRandomNumber (Math|Random|RandomIntegerinRange 0 5)))

(event Custom|StartSpinning
  (params (NumbersToDisplay :type Map%20of%20Integers%20to%20Integers))
  (bind _rollerstaticmesh (Variables|Default|GetRollerStaticMesh))
  (Variables|Result|SetRandomValue (- (.Value (Utilities|Map|Find NumbersToDisplay (Variables|InitialSetup|GetRollerId))) 1))
  (Utilities|FlowControl|Delay (Variables|InitialSetup|GetDelayStartSpining))
  (Utilities|FlowControl|DoOnce false
    (:Completed
      (Util|ResetRotation)
      (Class|PrimitiveComponent|SetAngularDamping _rollerstaticmesh (Variables|InitialSetup|GetAngularDamping))
      (Physics|SetSimulatePhysics _rollerstaticmesh true)
      (Class|PrimitiveComponent|AddTorque _rollerstaticmesh (Math|Vector|MakeVector 0.0 (Variables|InitialSetup|GetAngularSpeed) 0.0) "None" true)
      (Utilities|FlowControl|Delay 0.5)
      (CallFunction|StopSpining))))

(event Custom|StopWeel
  (if (Utilities|Time|IsValidTimerHandle (Variables|Spinning|GetStopWeelTimerHandler))
    (if (== (Variables|Spinning|GetIncrement) (Variables|Spinning|GetNumberOfSteps))
      ;[0.2806 0.5878 1] Reset Stop Weel
      (Utilities|Time|ClearandInvalidateTimerbyHandle (Variables|Spinning|GetStopWeelTimerHandler))
      (Variables|Spinning|SetIncrement 0)
      (Default|CallRollerStopped (Variables|InitialSetup|GetRollerId) (+ (Variables|Result|GetRandomValue) 1))
      (else
        ;[0.9073 0.552 1] Add rotating by sub steps
        (Transformation|AddWorldRotation (Variables|Default|GetRollerStaticMesh) (Math|Rotator|MakeRotator 0.0 (Variables|Spinning|GetSubSteps) 0.0) false false)
        (Math|Integer|IncrementInt (Variables|Spinning|GetIncrement))))))

(event Custom|CheckForFaceZero
  (if (and (Variables|Spinning|GetShouldStopSpining) (Math|Float|InRange(Float) (Class|KismetMathLibrary|DegAcos (Math|Vector|DotProduct (Math|Vector|GetForwardVector (Variables|Default|GetRefereceArrow)) (Math|Vector|GetForwardVector (Variables|Default|GetRotatingArrow)))) 0.0 1e+01))
    ;[1 0.753 0.4366] Stop Simulating Physics
    (Utilities|StopRotatingUsingPhysics)
    ;[0.2225 0.4386 0.5] Computes the number for sub steps that are necessary
    (Variables|Spinning|SetNumberOfSteps (Math|Float|Truncate (/ (Math|Conversions|ToFloat(Integer) (Variables|Spinning|GetStopAtAngle)) (Variables|Spinning|GetSubSteps))))
    (bind _returnvalue (Utilities|Time|SetTimerbyEvent (delegate Custom|StopWeel) (/ (Variables|Spinning|GetSubSteps) (Variables|Spinning|GetCurrentAngularSpeed)) true))
    (Variables|Spinning|SetStopWeelTimerHandler _returnvalue)))

(event EventBeginPlay
  (bind _asbp_spin_machine (Utilities|Casting|CastToBP_SpinMachine (Actor|GetParentActor)))
  (EventDispatchers|AssignStartRollers _asbp_spin_machine (delegate Custom|StartSpinning))
  (Physics|SetEnableGravity (Variables|Default|GetRollerStaticMesh) false)
  (Utilities|Time|SetTimerbyEvent (delegate Custom|GenerateRandomNumber) 0.02 true))

(event Collision|EventActorBeginOverlap
  (params (OtherActor :type Actor%20Object%20Reference)))

(event EventTick
  (params (DeltaSeconds :type Float%20%28single-precision%29)))

(fn ConstructionScript)

(fn ResetRotation
  (bind _rollerstaticmesh (Variables|Default|GetRollerStaticMesh))
  (bind _returnvalue (Transformation|GetWorldRotation _rollerstaticmesh))
  ;[0.2645 1 0.8496] Reset the rotation of the well
  (Transformation|SetRelativeRotation _rollerstaticmesh (Math|Rotator|MakeRotator (.roll _returnvalue) 0.0 (.yaw _returnvalue)) false false))

(fn GetRandom
  (return (Variables|Random|GetTempRandomNumber)))

(fn UpdateSpinStatus
  (if (Variables|InitialSetup|GetShouldUpdateSpin)
    ;[0.8864 0.6729 1] Update bool. If false return true, if true return false.
    (Variables|Spinning|SetShouldStopSpining (select (Variables|Spinning|GetShouldStopSpining) false true))))

(fn GetNumberOfFaces
  (return (Variables|InitialSetup|GetNumberOfFaces)))