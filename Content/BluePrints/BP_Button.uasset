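; Physical VR push button that a motion controller presses to trigger a linked Machine.
; A hit stops the button's physics, and hits aligned with its up axis play a timeline that sinks it and tints it red.
; A Detector overlap with the button calls ButtonPressed on the Machine, while SetButtonParent restores physics and attachment after animation.
; Construction creates dynamic materials for configurable base and button colors.
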(event OnComponentBeginOverlap(Detector)
  (params (OverlappedComponent :type Primitive%20Component%20Object%20Reference) (OtherActor :type Actor%20Object%20Reference) (OtherComp :type Primitive%20Component%20Object%20Reference) (OtherBodyIndex :type Integer) (bFromSweep :type Boolean) (SweepResult :type Hit%20Result%20Structure%20%28by%20ref%29))
  ;[0.2387 1 0.7881] When the button is pressed trigger the machine
  (if (== OtherComp (Variables|Default|GetButton))
    (Default|ButtonPressed (Variables|Setup|GetMachine))))

(event OnComponentHit(Button)
  (params (HitComponent :type Primitive%20Component%20Object%20Reference) (OtherActor :type Actor%20Object%20Reference) (OtherComp :type Primitive%20Component%20Object%20Reference) (NormalImpulse :type Vector) (Hit :type Hit%20Result%20Structure%20%28by%20ref%29))
  ;[0.4476 0.2572 1] Detect hit with the hand and start press animation
  (Utilities|Casting|CastToBP_MotionController OtherActor)
  (Utilities|FlowControl|DoOnce false :!label _label
    (:Completed
      (Physics|SetSimulatePhysics (Variables|Default|GetButton) false)
      (Components|Timeline|SetPlayRate (Variables|Default|GetPressButton) 4.0)
      (|PlayButtonAnimation (Math|Float|InRange(Float) (Math|Vector|DotProduct (* (Math|Vector|Normalize (.Normal (Collision|BreakHitResult Hit))) -1.0) (Math|Vector|GetUpVector (Variables|Default|GetButton))) 0.9 1.0))
      (goto _label Reset))))

(event EventBeginPlay
  (Utilities|SetButtonParent))

(event Collision|EventActorBeginOverlap
  (params (OtherActor :type Actor%20Object%20Reference)))

(event EventTick
  (params (DeltaSeconds :type Float%20%28single-precision%29)))

(fn ConstructionScript
  (bind _button (Variables|Default|GetButton))
  (bind _base (Variables|Default|GetBase))
  (Utilities|FlowControl|Sequence
    (:then_0
      ;[0.6523 1 0.9501] Sets the color for the Base
      (bind _returnvalue (Rendering|Material|CreateDynamicMaterialInstance _base 0 (Rendering|Material|GetMaterial _base 0) :!class /Script/Engine.PrimitiveComponent))
      (bind _output_get (Variables|Color|SetBaseMaterialInst _returnvalue))
      (Rendering|Material|SetVectorParameterValue _output_get (Variables|Color|GetBaseColorName) (Variables|Color|GetBaseColor) :!class /Script/Engine.MaterialInstanceDynamic))
    (:then_1
      ;[0.6523 1 0.9501] Sets the color for the button
      (bind _returnvalue_2 (Rendering|Material|CreateDynamicMaterialInstance _button 0 (Rendering|Material|GetMaterial _button 0) :!class /Script/Engine.PrimitiveComponent))
      (bind _output_get_2 (Variables|Color|SetButtonMaterialInst _returnvalue_2))
      (Rendering|Material|SetVectorParameterValue _output_get_2 (Variables|Color|GetButtonColorName) (Variables|Color|GetButtonColor) :!class /Script/Engine.MaterialInstanceDynamic))))