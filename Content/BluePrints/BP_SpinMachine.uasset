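; Slot machine actor that spins attached BP_Roller actors on a button press and evaluates the resulting combination.
; BPSCProbabilities picks the combination up front, which is mapped by roller ID before the rollers start.
; Each roller's stop event records its value and updates the next roller's spin status.
; Tick detects when all have stopped, matches the combination against WinTable rows, prints the win mode and resets the machine.
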(event Custom|RollerStoped
  (params (Id :type Integer) (Random%20Value :type Integer))
  ;[0.45 1 0.658] Bind the event for each roller
  ;;[0.1978 0.4971 1] Call when roller stop
  (CallFunction|SetStoppedRoller Id Random%20Value))

(event Custom|ButtonPressed
  ;[0.3588 1 0.3152] Here is the logic for start spinning
  (if (Variables|Default|GetisReadyToSpin)
    (Variables|Default|SetisReadyToSpin false)
    (bind _combination (Default|PickRandom (Variables|Default|GetBPSC_Probabilities))) ; Check If Player Won or Lost
    (Utilities|SetArrayIntoMap _combination
      (:Completed
        (Default|CallStartRollers (Variables|Default|GetRandomValue))))))

(event EventBeginPlay
  (bind _bpsc_probabilities (Variables|Default|GetBPSC_Probabilities))
  (bind _rollers (Variables|Rollers|GetRollers))
  (Variables|Default|SetisReadyToSpin true)
  (Utilities|Array|Clear (Variables|Rollers|GetRollers))
  (for _array_element (Actor|GetAttachedActors self)
    ;[0.4757 0.8169 1] Set the rollers into an array.
    (bind _asbp_roller (Utilities|Casting|CastToBP_Roller _array_element))
    (Utilities|Array|AddUnique (Variables|Rollers|GetRollers) _asbp_roller)
    ;[0.45 1 0.658] Bind the event for each roller
    (EventDispatchers|AssignRollerStopped _asbp_roller (delegate Custom|RollerStoped)))
  ;[0.4594 1 0.774] Set the number of Faces from one roller. PS: They should be all the same. Then set the number of rollers
  (Default|SetNumberOfFaces _bpsc_probabilities (Default|GetNumberOfFaces (Utilities|Array|Get(acopy) _rollers)))
  (Default|SetNumberOfRollers _bpsc_probabilities (Utilities|Array|Length _rollers)))

(event Collision|EventActorBeginOverlap
  (params (OtherActor :type Actor%20Object%20Reference)))

(event EventTick
  (params (DeltaSeconds :type Float%20%28single-precision%29))
  (if (== (Utilities|Map|Length (Variables|Default|GetisFinished)) (Utilities|Array|Length (Variables|Rollers|GetRollers)))
    ;[0.3181 1 0.7873] Comment
    (Utilities|Map|Clear (Variables|Default|GetisFinished))
    (Development|PrintString "All Rollers Stopped")
    (bind _result (CallFunction|CheckResult))
    (Development|PrintString (Utilities|String|EnumtoString (.WinMode (Utilities|Struct|BreakSWinTable _result))))
    ;[0.577 0.6334 1] Necessary sync full stop
    (Utilities|FlowControl|Delay 0.0) ; Wait to sync
    (bind _success_reset (CallFunction|ResetMachine))
    (Variables|Default|SetisReadyToSpin _success_reset)))

(fn ConstructionScript)

(fn SetStoppedRoller
  (params (Id :type Integer) (RandomValue :type Integer))
  (LocalVariables|SetLocalId Id)
  (LocalVariables|SetLocalRandom RandomValue)
  (Utilities|FlowControl|Sequence
    (:then_0
      ;[0.5948 0.8787 1] Dictonary for finished rollers
      (bind _returnvalue (Utilities|Map|Add (Variables|Default|GetisFinished) (LocalVariables|GetLocalId) true))
      (if (not _returnvalue)
        (Development|PrintString "Error...isFinisheDic Shoud be clean")))
    (:then_1
      ;[1 1 1] Dictonary with the random values
      (Utilities|Map|Add (Variables|Default|GetRandomValue) (LocalVariables|GetLocalId) (LocalVariables|GetLocalRandom))
      ;[0.765 0.6934 0.2199 0.363] Update Spin status
      (switch int (LocalVariables|GetLocalId)
        (:0
          ;;[0.59 1 0.814] Update the roller num 2
          (Default|UpdateSpinStatus (.AsBP%20Roller (Utilities|Casting|CastToBP_Roller (Variables|/Script/Engine.ChildActorComponent|GetChildActor (Variables|Default|GetRoller2))))))
        (:1
          ;;[0.59 1 0.814] Update the roller num 3
          (Default|UpdateSpinStatus (.AsBP%20Roller (Utilities|Casting|CastToBP_Roller (Variables|/Script/Engine.ChildActorComponent|GetChildActor (Variables|Default|GetRoller3))))))))))

(fn ResetMachine
  ;[0.272 1 0.5884] Enable all rollers to spin again
  (for _array_element (Variables|Rollers|GetRollers)
    (Default|EnableSpin _array_element)
    (Default|UpdateSpinStatus _array_element))
  (return true))

(fn CheckResult
  (bind _randomvalue (Variables|Default|GetRandomValue))
  ;[1 0.7303 0.5879] Debug node
  (Development|PrintText (Utilities|Text|FormatText "Combination of : {val0}, {val1}, {val2}" (.Value (Utilities|Map|Find _randomvalue 0)) (.Value (Utilities|Map|Find _randomvalue 1)) (.Value (Utilities|Map|Find _randomvalue 2))) true true "(R=1.000000,G=0.009947,B=0.000000,A=1.000000)" 5.0)
  (bind _outrownames (DataTable|GetDataTableRowNames (Variables|Default|GetWinTable)))
  (bind _array_element (Utilities|Array|ForEachLoopwithBreak _outrownames :!label _label)
    (:LoopBody
      ;[0 0.9254 1] Loop over all the lines on the WinTable
      (bind _returnvalue (Utilities|GetDataTableRow "/Game/DataTables/WinTable.WinTable" _array_element)
        (:then
          ;;[0.4724 0.3075 1] Assumes you always win
          (LocalVariables|SetisWinner true)
          (bind (_array_element_2 _array_index) (Utilities|Array|ForEachLoopwithBreak (.Combination (Utilities|Struct|BreakSWinTable _returnvalue)) :!label _label_2)
            (:LoopBody
              ;;[0.2746 0.5762 1] Loops over the 3 roller. If one is not equal exit it
              (if (not (== _array_element_2 (.Value (Utilities|Map|Find (Variables|Default|GetRandomValue) _array_index))))
                (LocalVariables|SetisWinner false)
                (goto _label_2 Break)))
            (:Completed
              ;;[0.3385 1 0.9202] After check all the roller, if isWinner is still true, then the combination is equal
              (if (LocalVariables|GetisWinner)
                (LocalVariables|SetReturnWin _returnvalue)
                (goto _label Break)))))
        (:RowNotFound
          (Development|PrintString "Warnning: Probably using wrong table."))))
    (:Completed
      ;[1 0.5395 0.9413] Return Result
      (if (LocalVariables|GetisWinner)
        (return (LocalVariables|GetReturnWin))
        (else
          (return (LocalVariables|GetReturnLose)))))))