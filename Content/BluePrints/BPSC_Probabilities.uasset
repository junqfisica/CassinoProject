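; Slot-machine probability Blueprint that decides whether a roll wins, along with its combination and euro prize.
; On BeginPlay it carves a number pool into per-row sets sized by each WinTable probability, leaving the remainder as losing numbers.
; PickRandom draws a number, and CheckResult returns the matching row's combination and value or builds a random losing combination.
; Losing combinations use AddUnique for the last face so it differs from the others.
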(event EventBeginPlay
  (bind _list (CallFunction|SetArraywithHundredElements))
  (Variables|Probability|SetGenerator _list)
  (Probability|SetDicsOfProbabilities))

(event EventTick
  (params (DeltaSeconds :type Float%20%28single-precision%29)))

(fn SetDicsOfProbabilities
  (Development|PrintString "StartFunc")
  ;[0.6208 1 0.8678] Get data from win table
  (bind _outrownames (DataTable|GetDataTableRowNames (Variables|DataTable|GetWinTable)))
  ;[0.333 0.9801 1 0.2] Loop over each row in the WinTable
  (for _array_element _outrownames
    (bind _output_get (LocalVariables|SetRowName _array_element))
    (Development|PrintString (Utilities|String|ToString(Name) _output_get))
    (bind _returnvalue (Utilities|GetDataTableRow "/Game/DataTables/WinTable.WinTable" _output_get)
      (:then
        (bind _result (Utilities|Set|ToArray (Variables|Probability|GetGenerator)))
        (LocalVariables|SetTempArray _result)
        (for _index (range 0 (- (Math|Float|Truncate (* (Variables|Probability|GetTotalSetOfNumbers) (.Probability (Utilities|Struct|BreakSWinTable _returnvalue)))) 1))
          ;;[0.6483 1 0.6033] Loop over the number of elemnts on the Generator and set a temporary list
          (Utilities|Set|Add (LocalVariables|GetTempList) (Utilities|Array|Get(acopy) (LocalVariables|GetTempArray) _index)))
        ;;[0.5462 1 0.9301] Add it to a dictionary that contains the Array of Probability
        (Utilities|Map|Add (Variables|Probability|GetDSetOfProbability) (LocalVariables|GetRowName) (Utilities|Struct|MakeSArrayOfProbability (LocalVariables|GetTempList)))
        (CallFunction|PrintIntegerList "TempList" (LocalVariables|GetTempList))
        ;;[0.5271 0.9401 1] Remove numbers from the Tempgenaretor
        (bind _result_2 (Utilities|Set|ToArray (LocalVariables|GetTempList)))
        (Utilities|Set|RemoveItems (Variables|Probability|GetGenerator) _result_2)
        (|LenghOfTempGenerator)
        (CallFunction|PrintIntegerList "Generator" (Variables|Probability|GetGenerator))
        ;;[0.523 0.7487 1] Clear temp list
        (Utilities|Set|Clear (LocalVariables|GetTempList))
        (Utilities|Array|Clear (LocalVariables|GetTempArray)))
      (:RowNotFound
        ;;[1 0.3959 0.3061] Error message
        (Development|PrintString "Warnning: Probably using wrong table.")))))

(fn CheckResult
  (params (ValuePicked :type Integer))
  (LocalVariables|SetLPickedValue ValuePicked)
  (if (Utilities|Set|Contains (Variables|Probability|GetGenerator) ValuePicked)
    (Development|PrintString "You Lost")
    (bind _combination (Result|BuildArrayforLooseCombination (Variables|Setup|GetNumberOfRollers) (Variables|Setup|GetNumberOfFaces)))
    (CallFunction|PrintIntegerArray "Fail" _combination)
    (return false _combination 0)
    (else
      (bind _keys (Utilities|Map|Keys (Variables|Probability|GetDSetOfProbability)))
      (bind _array_element (Utilities|Array|ForEachLoopwithBreak _keys)
        (:LoopBody
          (if (Utilities|Set|Contains (Utilities|Struct|BreakSArrayOfProbability (.Value (Utilities|Map|Find (Variables|Probability|GetDSetOfProbability) _array_element))) (LocalVariables|GetLPickedValue))
            (bind _returnvalue (Utilities|GetDataTableRow "/Game/DataTables/WinTable.WinTable" _array_element)
              (:then
                (|PrintResult (.Value (Utilities|Struct|BreakSWinTable _returnvalue)) (.WinMode (Utilities|Struct|BreakSWinTable _returnvalue)))
                (return true (.Combination (Utilities|Struct|BreakSWinTable _returnvalue)) (.Value (Utilities|Struct|BreakSWinTable _returnvalue)))))))
        (:Completed
          (Development|PrintString "No value match!! ")
          (return false (Utilities|Array|MakeArray 10) 0))))))

(fn BuildArrayforLooseCombination
  (params (CombinationSize :type Integer) (NumberOfFaces :type Integer))
  (LocalVariables|SetLNumberOfFaces NumberOfFaces)
  (for _index (range 0 (- CombinationSize 2))
    ;[0.5256 1 0.9301] Add N - 1 elements on the array
    (Utilities|Array|Add (LocalVariables|GetLCombination) (Math|Random|RandomIntegerinRange 1 (LocalVariables|GetLNumberOfFaces))))
  (while (!= CombinationSize (Utilities|Array|Length (LocalVariables|GetLCombination)))
    ;[1 0.3412 0.7222] Add the last element on the array. It must be unique.
    (Utilities|Array|AddUnique (LocalVariables|GetLCombination) (Math|Random|RandomIntegerinRange 1 (LocalVariables|GetLNumberOfFaces))))
  ;[0.5136 1 0.92 0.5] Return combination
  (return (LocalVariables|GetLCombination)))

(fn SetNumberOfFaces
  (params (NumberOfFaces :type Integer))
  (Variables|Setup|SetNumberOfFaces NumberOfFaces))

(fn SetNumberOfRollers
  (params (NumberOfFaces :type Integer))
  (Variables|Setup|SetNumberOfRollers NumberOfFaces))

(fn PickRandom
  (bind _output_get (Variables|Probability|SetPickedRandom (Math|Random|RandomInteger (Variables|Probability|GetTotalSetOfNumbers))))
  (Development|PrintText (Utilities|Text|FormatText "Number picked: {val}" _output_get))
  (bind (_iswinner _combination _value) (Probability|CheckResult (Variables|Probability|GetPickedRandom)))
  (return _iswinner _combination _value))